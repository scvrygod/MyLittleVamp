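; BP_Weapon_Mass is an area-of-effect weapon that damages everything around it when fired.
; FireEvent runs a zero-length multi sphere trace on the Visibility channel at its own location, ignoring itself and its owner, with debug drawing on.
; Each hit receives an IsEnemy interface call, but the following branch is constant true, so every hit gets Damage applied with the owner as causer.
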(event `self.FireEvent`
  (bind _returnvalue (`self.K2_GetActorLocation`))
  (bind (_outhits _returnvalue_2) (`KismetSystemLibrary.SphereTraceMulti` _returnvalue _returnvalue 500.0 "TraceTypeQuery1" false (`|MakeArray` self (`self.GetOwner`) :!type "Actor Object Reference") "ForDuration" true (struct :`R` 1.0) (struct :`G` 0.053862 :`B` 1.0 :`A` 1.0) 0.2))
  (if _returnvalue_2
    (for _array_element _outhits
      (bind (_bblockinghit _binitialoverlap _time _distance _location _impactpoint _normal _impactnormal _physmat _hitactor) (`GameplayStatics.BreakHitResult` _array_element))
      (message `/Game/MyGame/Blueprints/Interface/BPI_EnemyInterface.IsEnemy` _hitactor)
      (if true
        (`GameplayStatics.ApplyDamage` _hitactor (`self.Damage`) null (`self.GetOwner`))))))

(fn `UserConstructionScript`
  (`parent.UserConstructionScript`))