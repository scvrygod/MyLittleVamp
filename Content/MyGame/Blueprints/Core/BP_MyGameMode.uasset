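; Game mode that runs endless timed enemy waves around the player and provides a score award function.
; A looping timer calls SpawnEnemy with a growing count, placing enemies evenly on a circle around the pawn, skipping blocked spots.
; Spawned enemies gain health with the wave count, get a death event binding and are tracked in an array.
; The timer clears when the pawn is invalid; the all-enemies-dead check is disconnected.
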(event `self.ReceiveBeginPlay`
  (`self.StartSpawnTimer` 10.0))

(event `StartSpawnTimer`
  (params (Time :type "Float (double-precision)" :default 3.0))
  (bind _returnvalue (`KismetSystemLibrary.K2_SetTimerDelegate` (delegate `SpawnTick`) Time true))
  (set `self.SpawnTimer` _returnvalue))

(event `SpawnTick`
  (`self.SpawnEnemy` (`self.AmountOfEnemy`))
  (`/Engine/EditorBlueprintResources/StandardMacros.IncrementInt` (`self.AmountOfEnemy`)))

(fn `AddScore`
  (params (DamageController :type "Controller Object Reference"))
  (message `/Game/MyGame/Blueprints/Interface/BPI_PlayerState.AddScore` (`Controller.PlayerState` DamageController) 10))

(fn `CheckSpawnAvailable`
  (returns (bAvailableSpawn :type Boolean))
  (locals (L_Available :type Boolean))
  (set `local.L_Available` true)
  (for _array_element (`self.EnemyArray`)
    (`/Engine/EditorBlueprintResources/StandardMacros.IsValid` _array_element
      (:`Is Valid`
        (set `local.L_Available` false))))
  (return (`local.L_Available`)))

(fn `SpawnEnemy`
  (params (AmountEnemyonWave :type Integer))
  (bind _returnvalue (`GameplayStatics.GetPlayerPawn` 0))
  (bind (_returnvalue_x _returnvalue_y _returnvalue_z) (`KismetMathLibrary.BreakVector` (`self.K2_GetActorLocation` _returnvalue)))
  (for _index (range AmountEnemyonWave)
    (`/Engine/EditorBlueprintResources/StandardMacros.IsValid` _returnvalue
      (:`Is Valid`
        (bind _returnvalue_2 (`|SpawnActorFromClass` "/Game/MyGame/Blueprints/Enemy/BP_Enemy_Base.BP_Enemy_Base_C" (`KismetMathLibrary.MakeTransform` (+ (`KismetMathLibrary.GreaterGreater_VectorRotator` (`KismetMathLibrary.MakeVector` (`self.Radius`) 0.0 _returnvalue_z) (`KismetMathLibrary.MakeRotator` 0.0 0.0 (* _index (/ 360.0 (`KismetMathLibrary.Conv_IntToDouble` AmountEnemyonWave))))) (`self.K2_GetActorLocation` (`GameplayStatics.GetPlayerPawn` 0)))) "DontSpawnIfColliding" "OverrideRootScale" null null))
        (`/Engine/EditorBlueprintResources/StandardMacros.IsValid` _returnvalue_2
          (:`Is Valid`
            (set `/Game/MyGame/Blueprints/Enemy/BP_Enemy_Base.Health` (+ (`/Game/MyGame/Blueprints/Enemy/BP_Enemy_Base.Health` _returnvalue_2) (* (`KismetMathLibrary.Conv_IntToDouble` (`self.AmountOfEnemy`)) 2.0)) _returnvalue_2)
            (add `/Game/MyGame/Blueprints/Enemy/BP_Enemy_Base.EnemyDie` _returnvalue_2 (`|CreateDelegate` :!event `AddScore`))
            (`KismetArrayLibrary.Array_Add` (`self.EnemyArray`) _returnvalue_2))))
      (:`Is Not Valid`
        (`KismetSystemLibrary.K2_ClearAndInvalidateTimerHandle` (`self.SpawnTimer`))))))

(fn `UserConstructionScript`)