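; BP_Weapon_Speed is a weapon Blueprint whose level upgrades increase its rate of fire.
; It extends the parent's UpgradeWeaponLevel, raising ShotsPerSecond by a tenth of its current value so upgrades compound, then calls StartFireTimer.
; Each upgrade also prints the new rate on screen in long-lasting red debug text.
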(event `self.UpgradeWeaponLevel`
  (bind _shotspersecond (`self.ShotsPerSecond`))
  (`parent.UpgradeWeaponLevel`)
  (set `self.ShotsPerSecond` (+ _shotspersecond (/ _shotspersecond 10)))
  (`self.StartFireTimer`)
  (`KismetSystemLibrary.PrintString` (`KismetStringLibrary.Conv_IntToString` (`self.ShotsPerSecond`)) true true (struct :`R` 1.0 :`A` 1.0) 99.0))

(fn `UserConstructionScript`
  (`parent.UserConstructionScript`))