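; Base enemy that chases the player pawn, deals melee area damage and can drop loot when killed.
; A BeginPlay loop runs AIMoveTo; on arrival it pulses the Cube's scale and damages BP_MyPawn actors inside the Sphere, retrying after delays.
; AnyDamage depletes Health, then reports the death, randomly spawns a medkit or rarer weapon pickup, and destroys the actor.
; Timer-based overlap attack logic remains but is disconnected.
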(event `self.ReceiveBeginPlay`
  (bind _returnvalue (`GameplayStatics.GetPlayerPawn` 0))
  (`/Engine/EditorBlueprintResources/StandardMacros.IsValid` _returnvalue :!label _label
    (:`Is Valid`
      (`|AIMoveTo` self (0.0 0.0 0.0) _returnvalue
        (:`OnSuccess`
          (`SceneComponent.SetRelativeScale3D` (`self.Cube`) (1.2 1.2 1.2))
          (`|ExecutionSequence`
            (:`then_0`
              (`KismetSystemLibrary.Delay` 1.0)
              (`SceneComponent.SetRelativeScale3D` (`self.Cube`) (1.0 1.0 1.0))
              (`KismetSystemLibrary.Delay` 1.0)
              (goto _label))
            (:`then_1`
              (for _array_element (`PrimitiveComponent.GetOverlappingActors` (`self.Sphere`) "/Game/MyGame/Blueprints/Core/BP_MyPawn.BP_MyPawn_C")
                (`GameplayStatics.ApplyDamage` _array_element (`self.Base Damage`) null self)))))
        (:`OnFail`
          (`KismetSystemLibrary.Delay` 1.0)
          (goto _label))))
    (:`Is Not Valid`
      (`KismetSystemLibrary.Delay` 5.0)
      (goto _label))))

(event `self.Sphere.OnComponentBeginOverlap`
  (params (OverlappedComponent :type "PrimitiveComponent Object Reference") (OtherActor :type "Actor Object Reference") (OtherComp :type "PrimitiveComponent Object Reference") (OtherBodyIndex :type Integer) (bFromSweep :type Boolean) (SweepResult :type "HitResult Structure (by ref)")))

(event `AttackTick`)

(event `self.Sphere.OnComponentEndOverlap`
  (params (OverlappedComponent :type "PrimitiveComponent Object Reference") (OtherActor :type "Actor Object Reference") (OtherComp :type "PrimitiveComponent Object Reference") (OtherBodyIndex :type Integer)))

(event `self.ReceiveAnyDamage`
  (params (Damage :type "Float (single-precision)") (DamageType :type "DamageType Object Reference") (InstigatedBy :type "Controller Object Reference") (DamageCauser :type "Actor Object Reference"))
  (bind _output_get (set `self.Health` (- (`self.Health`) Damage)))
  (if (<= _output_get 0.0)
    (`self.EnemyDie` InstigatedBy)
    (`self.SpawnDrop`)
    (`self.K2_DestroyActor`)))

(event `SpawnDrop`
  (if (`KismetMathLibrary.RandomBoolWithWeight` 0.3)
    (if (`KismetMathLibrary.RandomBoolWithWeight` 0.1)
      (`|SpawnActorFromClass` "/Game/MyGame/Blueprints/World/BP_World_Weapon.BP_World_Weapon_C" (`KismetMathLibrary.MakeTransform` (`self.K2_GetActorLocation`)) "Undefined" "OverrideRootScale" null "/Game/MyGame/Blueprints/Weapon/BP_Weapon_Speed.BP_Weapon_Speed_C" true null)
      (else
        (`|SpawnActorFromClass` "/Game/MyGame/Blueprints/World/BP_World_MedKit.BP_World_MedKit_C" (`KismetMathLibrary.MakeTransform` (`self.K2_GetActorLocation`)) "Undefined" "OverrideRootScale" null 10.0 null)))))

(fn `IsEnemy`
  (returns (blsEnemy :type Boolean))
  (return true))

(fn `UserConstructionScript`)